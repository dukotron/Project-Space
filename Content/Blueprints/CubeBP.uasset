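; CubeBP is a clickable cube that acts as a selectable object in an RTS mechanics setup.
; BeginPlay caches the RTSMechanicsUI widget and player controller by searching all instances.
; Clicking the mesh while the UI's Loaded flag is false hides the current selection's components, then replaces the controller's SelectedObjects with this cube's Selected component.
; Tick re-shows everything in that shared list every frame.
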(event OnClicked(StaticMesh)
  (params (TouchedComponent :type Primitive%20Component%20Object%20Reference) (ButtonPressed :type Key%20Structure :default "AnyKey"))
  (bind _rtsmechanicsplayercontroller (Variables|Default|GetRTSMechanicsPlayerController))
  (bind _selectedobjects (Variables|/Game/Controllers/RTSMechanicsPlayerControllerBP.RTSMechanicsPlayerControllerBP_C|GetSelectedObjects _rtsmechanicsplayercontroller))
  (if (not (Variables|/Game/UI/RTSMechanicsUI.RTSMechanicsUI_C|GetLoaded (Variables|Default|GetRTSMechanicsUI)))
    (CallFunction|ApplyVisibility false)
    (Utilities|Array|Clear _selectedobjects)
    (Utilities|Array|Add _selectedobjects (Variables|Default|GetSelected))))

(event EventBeginPlay
  (bind _foundwidgets (Widget|GetAllWidgetsOfClass "/Game/UI/RTSMechanicsUI.RTSMechanicsUI_C" true))
  (for _array_element _foundwidgets
    _)
  (Variables|Default|SetRTSMechanicsUI _array_element)
  (bind _outactors (Actor|GetAllActorsOfClass "/Game/Controllers/RTSMechanicsPlayerControllerBP.RTSMechanicsPlayerControllerBP_C"))
  (for _array_element_2 _outactors
    _)
  (Variables|Default|SetRTSMechanicsPlayerController _array_element_2))

(event EventTick
  (params (DeltaSeconds :type Float%20%28single-precision%29))
  (CallFunction|ApplyVisibility true))

(fn ConstructionScript)

(fn ApplyVisibility
  (params (New%20Visibility :type Boolean))
  (for _array_element (Variables|/Game/Controllers/RTSMechanicsPlayerControllerBP.RTSMechanicsPlayerControllerBP_C|GetSelectedObjects (Variables|Default|GetRTSMechanicsPlayerController))
    (Rendering|SetVisibility _array_element New%20Visibility false)))