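; Player controller for the ship editor that creates and displays the ShipEditorUI widget and handles object placement input.
; PlaceObject spawns a CubeBP at the transform of the widget's SpawnedCube and ignores look input until the button is released.
; Cancel destroys that SpawnedCube and clears the widget's Loaded and Spawned flags.
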(event EventBeginPlay
  (bind _returnvalue (UserInterface|CreateWidget "/Game/UI/ShipEditorUI.ShipEditorUI_C"))
  (bind _output_get (Variables|Default|SetShipEditorUI _returnvalue))
  (UserInterface|Viewport|AddtoViewport _output_get 0))

(event Input|ActionEvents|InputActionPlaceObject
  (params (Key :type Key%20Structure :default "AnyKey"))
  (:Pressed
    (Input|SetIgnoreLookInput true)
    (Game|SpawnActorfromClass "/Game/Blueprints/CubeBP.CubeBP_C" (Transformation|GetActorTransform (Variables|/Game/UI/ShipEditorUI.ShipEditorUI_C|GetSpawnedCube (Variables|Default|GetShipEditorUI))) "Undefined" 0 0))
  (:Released
    (Input|ResetIgnoreLookInput)))

(event Input|ActionEvents|InputActionCancel
  (params (Key :type Key%20Structure :default "AnyKey"))
  (bind _shipeditorui (Variables|Default|GetShipEditorUI))
  (:Pressed
    (Variables|/Game/UI/ShipEditorUI.ShipEditorUI_C|SetLoaded _shipeditorui false)
    (Actor|DestroyActor (Variables|/Game/UI/ShipEditorUI.ShipEditorUI_C|GetSpawnedCube _shipeditorui))
    (Variables|/Game/UI/ShipEditorUI.ShipEditorUI_C|SetSpawned _shipeditorui false)))

(fn ConstructionScript)